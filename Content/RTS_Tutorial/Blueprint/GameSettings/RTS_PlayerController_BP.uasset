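; RTS player controller that drives the camera pawn, cast from the player pawn on BeginPlay, with zoom, rotation, movement and edge scrolling.
; Zoom changes spring arm length within limits, while holding Pan opens gates that let mouse axes rotate yaw and clamped pitch, suspending movement.
; Collapsed graphs handle swept axis movement at fixed height and viewport-edge scrolling, both scaled by a held speed modifier.
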(event EventBeginPlay
  (Utilities|ReferenceCast))

(event Input|ActionEvents|InputActionZoomReset
  (params (Key :type Key%20Structure :default "None"))
  ;[1 1 1] Zoom Controlls
  ;;[1 1 1] Zoom Reset
  (:Pressed
    (Variables|/Script/Engine.SpringArmComponent|SetTargetArmLength (Variables|/Game/RTS_Tutorial/Blueprint/GameSettings/RTS_CameraPawn_BP.RTS_CameraPawn_BP_C|GetSpringArm (Variables|Default|GetCameraPawnRef)) 1.5e+03)))

(event Input|ActionEvents|InputActionZoomIn
  (params (Key :type Key%20Structure :default "None"))
  (bind _camerapawnref (Variables|Default|GetCameraPawnRef))
  (bind _springarm (Variables|/Game/RTS_Tutorial/Blueprint/GameSettings/RTS_CameraPawn_BP.RTS_CameraPawn_BP_C|GetSpringArm _camerapawnref))
  ;[1 1 1] Zoom Controlls
  ;;[1 1 1] Zoom In
  (:Pressed
    (Variables|/Script/Engine.SpringArmComponent|SetTargetArmLength _springarm (Math|Float|Clamp(Float) (- (Variables|/Script/Engine.SpringArmComponent|GetTargetArmLength _springarm) (Variables|Zoom|GetZoomSpeed)) (Variables|Zoom|GetMinZoomLimit) (Variables|Zoom|GetMaxZoomLimit)))))

(event Input|ActionEvents|InputActionZoomOut
  (params (Key :type Key%20Structure :default "None"))
  (bind _camerapawnref (Variables|Default|GetCameraPawnRef))
  (bind _springarm (Variables|/Game/RTS_Tutorial/Blueprint/GameSettings/RTS_CameraPawn_BP.RTS_CameraPawn_BP_C|GetSpringArm _camerapawnref))
  ;[1 1 1] Zoom Controlls
  ;;[1 1 1] Zoom Out
  (:Pressed
    (Variables|/Script/Engine.SpringArmComponent|SetTargetArmLength _springarm (Math|Float|Clamp(Float) (+ (Variables|Zoom|GetZoomSpeed) (Variables|/Script/Engine.SpringArmComponent|GetTargetArmLength _springarm)) (Variables|Zoom|GetMinZoomLimit) (Variables|Zoom|GetMaxZoomLimit)))))

(event Input|ActionEvents|InputActionPan
  (params (Key :type Key%20Structure :default "None"))
  (bind _camerapawnref (Variables|Default|GetCameraPawnRef))
  (bind _returnvalue (Transformation|GetActorRotation _camerapawnref))
  (bind (_roll _pitch _yaw) (Math|Rotator|BreakRotator _returnvalue))
  ;[1 1 1] Pan Controlls
  ;;[1 1 1] Pan Y
  (:Pressed
    (Variables|Pan|SetDisablePanMovement true)
    (Utilities|FlowControl|Gate true) ; enters at Open
  )
  (:Released
    (Variables|Pan|SetDisablePanMovement false)
    (Utilities|FlowControl|Gate true) ; enters at Close
  ))

(event Input|ActionEvents|InputActionPan
  (params (Key :type Key%20Structure :default "None"))
  (bind _camerapawnref (Variables|Default|GetCameraPawnRef))
  (bind _returnvalue (Transformation|GetActorRotation _camerapawnref))
  (bind (_roll _pitch _yaw) (Math|Rotator|BreakRotator _returnvalue))
  ;[1 1 1] Pan Controlls
  ;;[1 1 1] Pan X
  (:Pressed
    (Variables|Pan|SetDisablePanMovement true)
    (Utilities|FlowControl|Gate true) ; enters at Open
  )
  (:Released
    (Variables|Pan|SetDisablePanMovement false)
    (Utilities|FlowControl|Gate true) ; enters at Close
  ))

(event Input|ActionEvents|InputActionPanReset
  (params (Key :type Key%20Structure :default "None"))
  (bind _camerapawnref (Variables|Default|GetCameraPawnRef))
  ;[1 1 1] Pan Controlls
  ;;[1 1 1] Pan Reset
  (:Pressed
    (Transformation|SetActorRotation _camerapawnref (Math|Rotator|MakeRotator (.Roll (Math|Rotator|BreakRotator (Transformation|GetActorRotation _camerapawnref))) 0.0 0.0))))

(event Input|ActionEvents|InputActionSpeedModifier
  (params (Key :type Key%20Structure :default "None"))
  ;[1 1 1] Movement Controls
  ;;[1 1 1] Set Movement modifier
  (:Pressed
    (Variables|Movement|SetMovementSpeedModifier 2.0))
  (:Released
    (Variables|Movement|SetMovementSpeedModifier 1.0)))

(event Input|AxisEvents|InputAxisMoveForward
  (params (AxisValue :type Float%20%28single-precision%29))
  ;[1 1 1] Movement Controls
  ;;[1 1 1] Basic Movement Controls
  (if (not (Variables|Pan|GetDisablePanMovement))
    (Utilities|BasicMovementControls AxisValue (stale Input|AxisEvents|InputAxisMoveRight AxisValue))))

(event Input|AxisEvents|InputAxisMoveRight
  (params (AxisValue :type Float%20%28single-precision%29))
  ;[1 1 1] Movement Controls
  ;;[1 1 1] Basic Movement Controls
  (if (not (Variables|Pan|GetDisablePanMovement))
    (Utilities|BasicMovementControls (stale Input|AxisEvents|InputAxisMoveForward AxisValue) AxisValue) ; enters at Right Movement
  ))

(event Input|MouseEvents|MouseX
  (params (AxisValue :type Float%20%28single-precision%29))
  ;[1 1 1] Movement Controls
  ;;[1 1 1] Edge Scroll Movement
  (if (not (Variables|Pan|GetDisablePanMovement))
    (bind (_deltaspeedx _deltaspeedy) (Utilities|EdgeScroll))
    (Transformation|AddActorLocalOffset (Variables|Default|GetCameraPawnRef) (Math|Vector|MakeVector _deltaspeedx _deltaspeedy 0.0) true false)))

(event Input|MouseEvents|MouseY
  (params (AxisValue :type Float%20%28single-precision%29))
  (bind _camerapawnref (Variables|Default|GetCameraPawnRef))
  (bind _returnvalue (Transformation|GetActorRotation _camerapawnref))
  (bind (_roll _pitch _yaw) (Math|Rotator|BreakRotator _returnvalue))
  ;[1 1 1] Pan Controlls
  ;;[1 1 1] Pan Y
  (Utilities|FlowControl|Gate true
    (:Exit
      (Transformation|SetActorRotation (Variables|Default|GetCameraPawnRef) (Math|Rotator|MakeRotator _roll (Math|Float|Clamp(Float) (+ _pitch (* AxisValue (Variables|Pan|GetPanSpeed))) -2e+01 5e+01) _yaw)))))

(event Input|MouseEvents|MouseX
  (params (AxisValue :type Float%20%28single-precision%29))
  (bind _camerapawnref (Variables|Default|GetCameraPawnRef))
  (bind _returnvalue (Transformation|GetActorRotation _camerapawnref))
  (bind (_roll _pitch _yaw) (Math|Rotator|BreakRotator _returnvalue))
  ;[1 1 1] Pan Controlls
  ;;[1 1 1] Pan X
  (Utilities|FlowControl|Gate true
    (:Exit
      (Transformation|SetActorRotation (Variables|Default|GetCameraPawnRef) (Math|Rotator|MakeRotator _roll _pitch (+ _yaw (* AxisValue (Variables|Pan|GetPanSpeed))))))))

(event Input|MouseEvents|MouseY
  (params (AxisValue :type Float%20%28single-precision%29))
  ;[1 1 1] Movement Controls
  ;;[1 1 1] Edge Scroll Movement
  (if (not (Variables|Pan|GetDisablePanMovement))
    (Utilities|EdgeScroll) ; enters at MouseY
  ))

(fn ConstructionScript)