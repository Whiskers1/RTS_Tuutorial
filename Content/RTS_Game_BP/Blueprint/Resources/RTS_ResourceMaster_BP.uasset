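; Base Blueprint for RTS resource objects that sets up each resource's amount and look in its Construction Script.
; A resource level, optionally randomized to exclude the zero-yield tier, selects a multiplier that turns the base amount into current resources.
; Optional flags randomize mesh scale independently per axis and world yaw, with rolls made whenever the Construction Script runs.
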(fn ConstructionScript
  (bind _minmeshsize (Variables|ResourceSize|GetMinMeshSize))
  (bind _maxmeshsize (Variables|ResourceSize|GetMaxMeshSize))
  (bind _returnvalue (Math|Random|RandomFloatinRange _minmeshsize _maxmeshsize))
  (if (Variables|Bool|GetIsRandomLevel)
    (bind _output_get (Variables|References|SetResourceLevelEnumRef (Utilities|Enum|ByteToEnumResourceLevelEnum (Math|Conversions|ToByte(Integer) (Math|Random|RandomIntegerinRange 1 6))))))
  (switch Utilities|FlowControl|Switch|SwitchonResourceLevelEnum _output_get
    (:NewEnumerator0
      (Variables|References|SetResourceModifier 0.0))
    (:NewEnumerator1
      (Variables|References|SetResourceModifier 1.0))
    (:NewEnumerator2
      (Variables|References|SetResourceModifier 1.2))
    (:NewEnumerator3
      (Variables|References|SetResourceModifier 1.4))
    (:NewEnumerator4
      (Variables|References|SetResourceModifier 1.6))
    (:NewEnumerator5
      (Variables|References|SetResourceModifier 1.8))
    (:NewEnumerator6
      (Variables|References|SetResourceModifier 2.0)))
  (Variables|ResourceValue|SetCurrentResources (* (Variables|ResourceValue|GetBaseResourceAmount) (Variables|References|GetResourceModifier)))
  (if (Variables|Bool|GetIsRandomSize)
    (Transformation|SetWorldScale3D (Variables|Default|GetResourceMesh) (Math|Vector|MakeVector _returnvalue _returnvalue _returnvalue)))
  (if (Variables|Bool|GetIsRandomRotated)
    (Transformation|SetWorldRotation (Variables|Default|GetResourceMesh) (Math|Rotator|MakeRotator 0.0 0.0 (Math|Random|RandomFloatinRange 0.0 3.6e+02)) false false)))