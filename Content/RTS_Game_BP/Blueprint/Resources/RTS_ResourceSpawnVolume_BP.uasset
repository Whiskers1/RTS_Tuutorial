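; RTS resource spawn volume that scatters resource actors at randomized spots derived from its bounds.
; On BeginPlay it can spawn a batch, then optionally start a looping timer for further batches until the running total reaches a maximum.
; SpawnResource box-traces on Visibility for each attempt and spawns only where the hit actor is a Landscape.
; The total counts requested amounts, including failed attempts.
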(event Custom|SpawnResourcesOnTimer
  (if (and (Variables|Bool|GetIsSpawnedOnTimer) (< (Variables|ResourceSettings|GetTotalNumberSpawned) (Variables|ResourceSettings|GetMaxResourcesSpawned)))
    (CallFunction|SpawnResource (Variables|References|GetResourceRef) (Variables|ResourceSettings|GetNumOfResourcesSpawnd))
    (Variables|ResourceSettings|SetTotalNumberSpawned (+ (Variables|ResourceSettings|GetNumOfResourcesSpawnd) (Variables|ResourceSettings|GetTotalNumberSpawned)))))

(event EventBeginPlay
  (if (Variables|Bool|GetIsSpawnedOnBeginPlay)
    (CallFunction|SpawnResource (Variables|References|GetResourceRef) (Variables|ResourceSettings|GetNumOfResourcesSpawnd))
    (Variables|ResourceSettings|SetTotalNumberSpawned (+ (Variables|ResourceSettings|GetNumOfResourcesSpawnd) (Variables|ResourceSettings|GetTotalNumberSpawned)))
    (if (and (Variables|Bool|GetIsSpawnedOnTimer) (< (Variables|ResourceSettings|GetTotalNumberSpawned) (Variables|ResourceSettings|GetMaxResourcesSpawned)))
      (Utilities|Time|SetTimerbyEvent (EventDispatchers|CreateEvent :!event Custom|SpawnResourcesOnTimer) (Variables|ResourceSettings|GetRespawnTime) true))))

(fn ConstructionScript)

(fn SpawnResource
  (params (Resource :type RTS%20Resource%20Master%20BP%20Class%20Reference) (SpawnAmount :type Integer))
  (bind (_origin _boxextent) (Collision|GetActorBounds false))
  (bind _z (Math|Vector|BreakVector _origin))
  (bind (_x _y) (Math|Vector|BreakVector _boxextent))
  (bind _returnvalue (* _y 2.0))
  (bind _returnvalue_2 (* _x 2.0))
  (bind _returnvalue_3 (- _y _returnvalue))
  (bind _returnvalue_4 (- _x _returnvalue_2))
  (bind _returnvalue_5 (Math|Random|RandomFloatinRange _returnvalue_3 _y))
  (bind _returnvalue_6 (Math|Random|RandomFloatinRange _returnvalue_4 _x))
  (bind _returnvalue_7 (Math|Vector|MakeVector _returnvalue_6 _returnvalue_5 _z))
  (bind _returnvalue_8 (+ _origin _returnvalue_7))
  (LocalVariables|SetResourceRefLocal Resource)
  (bind _output_get (LocalVariables|SetSpawnAmountLocal SpawnAmount))
  (for _index (range 0 _output_get)
    (bind _outhit (Collision|BoxTraceByChannel (+ _returnvalue_8 "0, 0,200.000000") "0, 0, 0" (- _returnvalue_8 "0, 0,200.000000") "0, 0, 0" "TraceTypeQuery1" false 0 "None"))
    (if (== (Utilities|GetClass (.HitActor (Collision|BreakHitResult _outhit))) "/Script/Landscape.Landscape")
      (Game|SpawnActorfromClass (LocalVariables|GetResourceRefLocal) (Math|Conversions|ToTransform(Vector) (.Location (Collision|BreakHitResult _outhit))) "Undefined" 0 0))))